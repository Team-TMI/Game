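; BP_RotSpike is an obstacle prop that swings back and forth in yaw about its PivotScene component.
; SwingHammer plays a timeline that interpolates the pivot's relative yaw across a half-turn arc.
; When the timeline finishes, its direction selects ReverseSwingHammer or SwingHammer, so the swing loops endlessly once started.
; BeginPlay is disabled and nothing in this graph makes the initial SwingHammer call.
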(event `self.SwingHammer`
  (set `self.Direction` "Forward")
  (bind (_direction _newtrack_0) (`Timeline|Timeline_0` :!label _label)
    (:`Update`
      (`SceneComponent.K2_SetRelativeRotation` (`self.PivotScene`) (`KismetMathLibrary.MakeRotator` 0.0 0.0 (`KismetMathLibrary.Lerp` -90.0 90.0 _newtrack_0)) false false))
    (:`Finished`
      (if (`|EnumEquality` _direction "Forward")
        (`self.ReverseSwingHammer`)
        (else
          (`self.SwingHammer`))))))

(event `self.ReverseSwingHammer`
  (set `self.Direction` "Backward")
  (goto _label :!via `Reverse`))

(fn `UserConstructionScript`)