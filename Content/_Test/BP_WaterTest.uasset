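; Test water volume actor that switches an overlapping BP_Frog between swimming, shallow-water and walking states.
; Entering Box starts the frog's swim and sets its movement mode to Flying.
; Entering Box1 stops swimming and flags Shallow while keeping Flying, and leaving Box1 clears the flag and restores Walking.
; Leaving Box does nothing, so the return to walking depends on exiting Box1.
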(event `self.Box.OnComponentBeginOverlap`
  (params (OverlappedComponent :type "PrimitiveComponent Object Reference") (OtherActor :type "Actor Object Reference") (OtherComp :type "PrimitiveComponent Object Reference") (OtherBodyIndex :type Integer) (bFromSweep :type Boolean) (SweepResult :type "HitResult Structure (by ref)"))
  (bind _asbp_frog (cast `/Game/Characters/BP_Frog` OtherActor))
  (`Frog.StartSwim` _asbp_frog)
  (`CharacterMovementComponent.SetMovementMode` (`Character.CharacterMovement` _asbp_frog) "MOVE_Flying" 0))

(event `self.Box.OnComponentEndOverlap`
  (params (OverlappedComponent :type "PrimitiveComponent Object Reference") (OtherActor :type "Actor Object Reference") (OtherComp :type "PrimitiveComponent Object Reference") (OtherBodyIndex :type Integer)))

(event `self.Box1.OnComponentBeginOverlap`
  (params (OverlappedComponent :type "PrimitiveComponent Object Reference") (OtherActor :type "Actor Object Reference") (OtherComp :type "PrimitiveComponent Object Reference") (OtherBodyIndex :type Integer) (bFromSweep :type Boolean) (SweepResult :type "HitResult Structure (by ref)"))
  (bind _asbp_frog (cast `/Game/Characters/BP_Frog` OtherActor))
  (set `/Game/Characters/BP_Frog.shallow` true _asbp_frog)
  (`Frog.StopSwim` _asbp_frog)
  (`CharacterMovementComponent.SetMovementMode` (`Character.CharacterMovement` _asbp_frog) "MOVE_Flying" 0))

(event `self.Box1.OnComponentEndOverlap`
  (params (OverlappedComponent :type "PrimitiveComponent Object Reference") (OtherActor :type "Actor Object Reference") (OtherComp :type "PrimitiveComponent Object Reference") (OtherBodyIndex :type Integer))
  (bind _asbp_frog (cast `/Game/Characters/BP_Frog` OtherActor))
  (`Frog.StopSwim` _asbp_frog)
  (`CharacterMovementComponent.SetMovementMode` (`Character.CharacterMovement` _asbp_frog) "MOVE_Walking" 0)
  (set `/Game/Characters/BP_Frog.shallow` false _asbp_frog))

(fn `UserConstructionScript`)