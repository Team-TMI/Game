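; BP_Thunder is a lightning effect that flashes repeatedly at random intervals while the game runs.
; BeginPlay starts an endless Delay loop that calls Strike after a random one-to-two-second wait, plus a short fixed pause between cycles.
; Strike replays the ThunderStrike timeline, whose tracks drive the Length and Emissive material parameters on ThunderPlane.
; Post-process settings nodes are present but never run.
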(event `self.ReceiveBeginPlay`
  (`KismetSystemLibrary.Delay` (`KismetMathLibrary.RandomFloatInRange` 1.0 2.0) :!label _label)
  (`self.Strike`)
  (`KismetSystemLibrary.Delay` 0.2)
  (goto _label))

(event `Strike`
  (bind _thunder_plane (`self.Thunder_Plane`))
  (bind (_direction _length _thunder) (`Timeline|ThunderStrike` :!via `PlayFromStart`)
    (:`Update`
      (`MeshComponent.SetScalarParameterValueOnMaterials` _thunder_plane "Length" _length)
      (`MeshComponent.SetScalarParameterValueOnMaterials` _thunder_plane "Emissive" _thunder))))

(fn `UserConstructionScript`)